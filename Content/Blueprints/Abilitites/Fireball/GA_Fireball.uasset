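; GA_Fireball is a Gameplay Ability that casts a fireball from a BP_Character.
; After committing, it plays the cast montage and immediately spawns a BP_Projectile attached to the character's right-hand socket.
; A montage notify detaches the projectile and launches it along the character's forward vector at the projectile speed.
; The ability ends when the montage completes, blends out or is interrupted, and cancels if the cast or commit fails.
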(event `self.K2_ActivateAbility`
  (bind _returnvalue_owneractor (break `GameplayAbilityActorInfo` (`self.GetActorInfo`)))
  (bind _asbp_character (cast `/Game/Blueprints/Character/BP_Character` _returnvalue_owneractor)
    (:`then`
      (set `self.CharacterRef` _asbp_character)
      (bind _returnvalue (`self.K2_CommitAbility`))
      (if _returnvalue
        (`|PlayMontage` (`Character.Mesh` (`self.CharacterRef`)) "/Game/Retarget/Anim_CastFireball.Anim_CastFireball"
          (:`then`
            (bind (_asynctaskproxy _spawnedactor) (`AbilityTask_SpawnActor.SpawnActor` (struct) "/Game/Blueprints/Abilitites/Fireball/BP_Projectile.BP_Projectile_C" (`self.CharacterRef`))
              (:`then`
                (bind _asbp_projectile (cast `/Game/Blueprints/Abilitites/Fireball/BP_Projectile` _spawnedactor))
                (bind _output_get (set `self.ProjectileRef` _asbp_projectile))
                (`Actor.K2_AttachToActor` _output_get (`self.CharacterRef`) "hand_rSocket" "KeepRelative" "KeepRelative" "KeepRelative" true))))
          (:`OnCompleted`
            (`self.K2_EndAbility` :!label _label))
          (:`OnBlendOut`
            (goto _label))
          (:`OnInterrupted`
            (goto _label))
          (:`OnNotifyBegin`
            (bind _projectileref (`self.ProjectileRef`)
              (:`then`
                (`Actor.K2_DetachFromActor` _projectileref "KeepRelative" "KeepRelative" "KeepRelative")
                (`/Game/Blueprints/Abilitites/Fireball/BP_Projectile.InitProjectileMovement` (`self.ProjectileRef`) (* (`Actor.GetActorForwardVector` (`self.CharacterRef`)) (`self.ProjectileSpeed`))))
              (:`else`))))
        (else
          (`self.K2_CancelAbility` :!label _label_2))))
    (:`CastFailed`
      (goto _label_2))))